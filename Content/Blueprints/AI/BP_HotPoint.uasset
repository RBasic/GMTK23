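; BP_HotPoint is an AI point marker that groups the BP_SubPoint actors lying within its zone.
; Its construction script scales PreviewRadius from RadiusZone, then rebuilds SubPoints from all BP_SubPoint actors within half of RadiusZone, so RadiusZone acts as a diameter.
; The event graph holds only disabled stubs, so the Blueprint adds no runtime logic.
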(event EventBeginPlay)

(event Collision|EventActorBeginOverlap
  (params (OtherActor :type Actor%20Object%20Reference)))

(event EventTick
  (params (DeltaSeconds :type Float%20%28single-precision%29)))

(fn ConstructionScript
  (Transformation|SetWorldScale3D (Variables|Default|GetPreviewRadius) (Math|Conversions|ToVector(Float) (/ (Variables|Default|GetRadiusZone) 1e+02)))
  (Utilities|Array|Clear (Variables|Default|GetSubPoints))
  (bind _outactors (Actor|GetAllActorsOfClass "/Game/Blueprints/AI/BP_SubPoint.BP_SubPoint_C"))
  (for _array_element _outactors
    (if (<= (Math|Vector|Distance(Vector) (Transformation|GetActorLocation _array_element) (Transformation|GetActorLocation)) (/ (Variables|Default|GetRadiusZone) 2.0))
      (Utilities|Array|AddUnique (Variables|Default|GetSubPoints) _array_element))))