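; Ghost AI character that performs evidence interactions (EMF, spirit box, fingerprints, D.O.T.S) for the player to discover as proofs.
; A timer runs the highest-weighted interaction from a random set kept unique across ghosts, raising the others' weights each round.
; Tick validates proofs and feeds an insanity value into smoke, mesh opacity and heartbeat audio.
; During the player's ult it flees through a blackboard flag and can be killed by clicking.
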(event OnComponentBeginOverlap(Sphere)
  (params (OverlappedComponent :type Primitive%20Component%20Object%20Reference) (OtherActor :type Actor%20Object%20Reference) (OtherComp :type Primitive%20Component%20Object%20Reference) (OtherBodyIndex :type Integer) (bFromSweep :type Boolean) (SweepResult :type Hit%20Result%20Structure%20%28by%20ref%29))
  (Utilities|Casting|CastToBP_Player OtherActor
    (:then
      (Variables|Default|SetcanHearSpiritBox true))
    (:CastFailed
      (bind _asbp_book (Utilities|Casting|CastToBP_Book OtherActor))
      (Utilities|Array|AddUnique (Variables|Default|GetbooksActivated) _asbp_book))))

(event OnComponentEndOverlap(Sphere)
  (params (OverlappedComponent :type Primitive%20Component%20Object%20Reference) (OtherActor :type Actor%20Object%20Reference) (OtherComp :type Primitive%20Component%20Object%20Reference) (OtherBodyIndex :type Integer))
  (Utilities|Casting|CastToBP_Player OtherActor
    (:then
      (Variables|Default|SetcanHearSpiritBox false))
    (:CastFailed
      (bind _asbp_book (Utilities|Casting|CastToBP_Book OtherActor))
      (Utilities|Array|RemoveItem (Variables|Default|GetbooksActivated) _asbp_book))))

(event Custom|ResetCanBeAfraidOfLittleInteract
  (Utilities|FlowControl|Delay 1e+01)
  (Variables|Default|Setb_canBeAfraidByLittleInteraction true))

(event Custom|SwitchInteractions
  (Utilities|Map|Clear (Variables|Default|GetInteractions))
  (Utilities|Time|PauseTimerbyHandle (Variables|Default|GetSwitchInteractionHandler))
  (CallFunction|SelectInteractions)
  (Default|Test (.AsWG%20Debug%20Interact (Utilities|Casting|CastToWG_DebugInteract (UserInterface|GetUserWidgetObject (Variables|Default|GetWidget)))) "Switching")
  (Utilities|FlowControl|Delay 7.0)
  (Development|PrintString "EEndSwitching !")
  (Utilities|Time|UnpauseTimerbyHandle (Variables|Default|GetSwitchInteractionHandler))
  (Variables|Default|SetWantsToSwitchInteractions false))

(event Custom|playerIsActive
  (Variables|Default|SetEMFPitchShift (Math|Float|MapRangeClamped (Math|Conversions|ToFloat(Integer) (Variables|/Game/Blueprints/Core/BP_Player.BP_Player_C|Geti_EMFSoundMax (Variables|Default|GetPlayerRef))) 0.0 5.0 0.0 1.5)))

(event Custom|WaitSpecialInteraction
  (params (Duration :type Float%20%28single-precision%29) (DotsRef :type BP%20DOTS%20Object%20Reference))
  (Utilities|FlowControl|Delay Duration)
  (Utilities|IsValid DotsRef
    (:Is%20Valid
      (Actor|DestroyActor DotsRef)
      (Variables|Default|SetdotsActivated 0))
    (:Is%20Not%20Valid
      _))
  (Variables|Default|SetWantsSpecialInteraction false)
  (CallFunction|LaunchInteraction)
  (bind _returnvalue (Utilities|Time|SetTimerbyFunctionName 0 "LaunchInteraction" (Variables|Default|GetTimeBetweenInteractions) true 0.0 (Variables|Default|GetInitial%20Start%20Delay%20Variance)))
  (Variables|Default|SetSwitchInteractionHandler _returnvalue))

(event EventTick
  (params (DeltaSeconds :type Float%20%28single-precision%29))
  (CallFunction|ManageSanity "NewEnumerator0" (* DeltaSeconds (select (Variables|Default|GetdebugMode) 0.0 0.001)))
  (CallFunction|ManageFreeze 0.02)
  (CallFunction|ManageRendering)
  (CallFunction|ManageInteractionsTick)
  (CallFunction|ManageAudio)
  (CallFunction|RunAway))

(event EventBeginPlay
  (CallFunction|InitializeAI)
  (CallFunction|SelectInteractions)
  (CallFunction|LaunchInteraction)
  (bind _returnvalue (Utilities|Time|SetTimerbyFunctionName 0 "LaunchInteraction" (Variables|Default|GetTimeBetweenInteractions) true 0.0 (Variables|Default|GetInitial%20Start%20Delay%20Variance)))
  (Variables|Default|SetSwitchInteractionHandler _returnvalue))

(event EventIsClick
  (params (fromMonster :type Boolean) (shouldSpawnFingerprint :type Boolean))
  (bind _playerref (Variables|Default|GetPlayerRef))
  (if (and (not (Variables|Default|GetIsDead)) (Variables|/Game/Blueprints/Core/BP_Player.BP_Player_C|Getb_inUlt _playerref))
    (Class|Pawn|DetachfromControllerPendingDestroy)
    (Default|StopFeedBackUlt _playerref)
    (Variables|Default|SetIsDead true)
    (CallFunction|ManageSanity "NewEnumerator4" 1.0)
    (CallFunction|ManageRendering)
    (Physics|SetSimulatePhysics (Variables|Character|GetMesh) true)
    (Actor|Tick|SetActorTickEnabled false)))

(fn ConstructionScript)

(fn SelectInteractions
  (LocalVariables|SetRandomNumberInteract (Math|Random|RandomIntegerinRange 0 2))
  (bind _enumvalue (|ForEachEPossibleInteractions)
    (:LoopBody
      (if (Math|Boolean|ANDBoolean (< (LocalVariables|GetAddCount) (LocalVariables|GetRandomNumberInteract)) (Utilities|Enum|NotEqual(Enum) _enumvalue "NewEnumerator3") (Utilities|Enum|NotEqual(Enum) _enumvalue "NewEnumerator5") (Utilities|Enum|NotEqual(Enum) _enumvalue "NewEnumerator7"))
        (bind _canadd (CallFunction|DetermineNewInteraction _enumvalue))
        (if _canadd
          (Math|Integer|IncrementInt (LocalVariables|GetAddCount)
            (:%20%20
              (Utilities|Map|Add (Variables|Default|GetInteractions) _enumvalue (Math|Random|RandomFloatinRange 0.0 1.0)))))))
    (:then
      (Utilities|Map|Add (Variables|Default|GetInteractions) "NewEnumerator7" (Math|Random|RandomFloatinRange 0.0 1.0)))))

(fn LaunchInteraction
  (bind _interactions (Variables|Default|GetInteractions))
  (bind _interactions_2 (Variables|Default|GetInteractions))
  (if (Variables|Default|GetWantsSpecialInteraction)
    (bind _outactors (Actor|GetAllActorsOfClass "/Game/Blueprints/Interactible/BP_Book.BP_Book_C"))
    (bind _returnvalue (Actor|GetActorOfClass "/Game/Blueprints/Interactible/BP_DOTS.BP_DOTS_C"))
    (bind _output_get (Variables|Default|SetCurrentInteraction (Utilities|Select :Index (Math|Random|RandomInteger 2) :Option%200 (select (not (Utilities|IsValid _returnvalue)) "NewEnumerator5" "NewEnumerator7") :Option%201 (select (< (Utilities|Array|Length _outactors) 2) "NewEnumerator5" "NewEnumerator7"))))
    (if (Utilities|Enum|Equal(Enum) _output_get "NewEnumerator7")
      (bind _keys (Utilities|Map|Keys _interactions_2 :!label _label))
      (bind _values (Utilities|Map|Values _interactions_2))
      (LocalVariables|SetIndexInteraction (.IndexOfMaxValue (Math|Float|MaxOfFloatArray _values)))
      (Variables|Default|SetCurrentInteraction (select (Variables|Default|GetdebugMode) (Variables|Default|GetCurrentInteraction) (Utilities|Array|Get(acopy) _keys (.IndexOfMaxValue (Math|Float|MaxOfFloatArray _values)))))
      (bind _keys_2 (Utilities|Map|Keys _interactions))
      (bind _values_2 (Utilities|Map|Values _interactions))
      (for (_array_element _array_index) _keys_2
        (Utilities|Map|Add (Variables|Default|GetInteractions) _array_element (Math|Float|Clamp(Float) (select (== _array_index (LocalVariables|GetIndexInteraction)) 0.0 (+ (Utilities|Array|Get(acopy) _values_2 _array_index) (Math|Random|RandomFloatinRange 0.1 0.15))))))
      (else
        (Utilities|Time|ClearandInvalidateTimerbyHandle (Variables|Default|GetSwitchInteractionHandler))
        (Development|PrintString (Utilities|String|Append "SPECIAL INTERACT : " (Utilities|String|EnumtoString _output_get)))))
    (else
      (goto _label)))
  (Default|Test (.AsWG%20Debug%20Interact (Utilities|Casting|CastToWG_DebugInteract (UserInterface|GetUserWidgetObject (Variables|Default|GetWidget)))) (Utilities|Text|ToText(String) (Utilities|String|EnumtoString (Variables|Default|GetCurrentInteraction))))
  (CallFunction|ManageInteractionsEnd)
  (Variables|Default|SetLastInteraction (Variables|Default|GetCurrentInteraction))
  (CallFunction|ManageInteractionsBegin))

(fn ManageSanity
  (params (State :type E_fManagerState%20Enum :default "NewEnumerator0") (Value :type Float%20%28double-precision%29))
  (switch Utilities|FlowControl|Switch|SwitchonE_fManagerState State
    (:NewEnumerator0
      (Variables|Default|SetInsanity (Math|Float|Clamp(Float) (+ (Variables|Default|GetInsanity) Value))))
    (:NewEnumerator1
      _)
    (:NewEnumerator4
      (Variables|Default|SetInsanity Value))
    (:NewEnumerator2
      (Variables|Default|SetInsanity 0.0)))
  (return (Variables|Default|GetInsanity)))

(fn ManageRendering
  (bind _insanity (Variables|Default|GetInsanity))
  (bind _returnvalue (<= _insanity 0.75))
  (bind _returnvalue_2 (select _returnvalue _insanity 0.0))
  (Utilities|FlowControl|Sequence
    (:then_0
      (Niagara|SetNiagaraVariable(Float) (Variables|Default|GetNS_Smoke) "Visibility" _returnvalue_2)
      (Niagara|SetNiagaraVariable(Float) (Variables|Default|GetNS_Smoke) "Rate" _returnvalue_2))
    (:then_1
      (Rendering|Material|SetScalarParameterValueonMaterials (Variables|Character|GetMesh) "Opacity" (Math|Float|MapRangeClamped (Variables|Default|GetInsanity) 0.7 1.0 0.0 2.0)))))

(fn ManageFreeze
  (params (FreezeValue :type Float%20%28double-precision%29))
  (CallFunction|ManageSanity "NewEnumerator0" (select (Variables|Default|GetFreezing) (* (Utilities|Time|GetWorldDeltaSeconds) FreezeValue) 0.0)))

(fn ManageAudio
  (bind _heartbeatsanity (Variables|Default|GetHeartBeatSanity))
  (bind _emfsound (Variables|Default|GetEMFSound))
  (Audio|Parameter|SetFloatParameter _heartbeatsanity "SanityPitch" (Math|Float|MapRangeClamped (Variables|Default|GetInsanity) 0.0 1.0 0.0 5.0) :!class /Script/AudioExtensions.AudioParameterControllerInterface)
  (Audio|Parameter|SetFloatParameter _heartbeatsanity "SanityGain" (Math|Float|MapRangeClamped (Variables|Default|GetInsanity) 0.0 1.0 0.0 3.0) :!class /Script/AudioExtensions.AudioParameterControllerInterface)
  (switch Utilities|FlowControl|Switch|SwitchonEPossibleInteractions (Variables|Default|GetCurrentInteraction)
    (:NewEnumerator2
      (Audio|Parameter|SetFloatParameter _emfsound "EMFPitch" (* (Variables|Default|GetNormalizedDistanceToPlayer) (Variables|Default|GetEMFPitchShift)) :!class /Script/AudioExtensions.AudioParameterControllerInterface)
      (Audio|Parameter|SetFloatParameter _emfsound "EMFGain" (Variables|Default|GetNormalizedDistanceToPlayer) :!class /Script/AudioExtensions.AudioParameterControllerInterface))))

(fn ManageInteractionsTick
  (bind _returnvalue (Transformation|GetActorLocation))
  (bind _playerref (Variables|Default|GetPlayerRef))
  (Utilities|FlowControl|Sequence
    (:then_0
      (switch Utilities|FlowControl|Switch|SwitchonEPossibleInteractions (Variables|Default|GetCurrentInteraction)
        (:NewEnumerator2
          (Variables|Default|SetNormalizedDistanceToPlayer (Math|Float|MapRangeClamped (Transformation|GetDistanceTo self _playerref) 5e+01 (Variables|/Game/Blueprints/Core/BP_Player.BP_Player_C|Getf_EMFMaxSoundRadius _playerref) 1.0 0.0)))
        (:NewEnumerator0
          (bind _outhit (Collision|SphereTraceForObjects _returnvalue _returnvalue 2.5e+02 (Utilities|Array|MakeArray "ObjectTypeQuery3") false 0 "None"))
          (bind _asbp_player (Utilities|Casting|CastToBP_Player (.hitactor _outhit)))
          (if (Variables|/Game/Blueprints/Core/BP_Player.BP_Player_C|Getscreaming _asbp_player)
            (CallFunction|ManageSanity "NewEnumerator0" (* 0.3 (Utilities|Time|GetWorldDeltaSeconds)))
            (Variables|Default|Setb_hasHearedSpirit true)))))
    (:then_1
      (CallFunction|CheckValidateProof))))

(fn ManageInteractionsBegin
  (bind _scene (Variables|Default|GetScene))
  (bind _returnvalue (Transformation|GetWorldLocation _scene))
  (switch Utilities|FlowControl|Switch|SwitchonEPossibleInteractions (Variables|Default|GetCurrentInteraction)
    (:NewEnumerator2
      (Audio|Components|Audio|Play (Variables|Default|GetEMFSound) 0.0))
    (:NewEnumerator0
      (bind _returnvalue_2 (Audio|SpawnSoundatLocation "/Game/Audio/Assets/AI/AI_VOX_Hunt/Vox_Hunt_000.Vox_Hunt_000" (Transformation|GetWorldLocation (Variables|Character|GetMesh)) "0, 0, 0" 1.0 1.0 0.0 0 0 :!label _label))
      (Effects|Components|ParticleSystem|SetIntParameter _returnvalue_2 "SwitchAIVocal" (Variables|Default|GetindexVoiceLine))
      (bind _output_get (Variables|Default|SetPlay%20IAVoice _returnvalue_2))
      (Audio|Components|Audio|Play _output_get 0.0)
      (Components|Activation|Activate (Variables|Default|GetNS_Disto) true))
    (:NewEnumerator4
      (Rendering|SetVisibility (Variables|Default|GetSpotLight) true false)
      (goto _label))
    (:NewEnumerator3
      (Game|SpawnActorfromClass "/Game/Blueprints/Interactible/BP_Book.BP_Book_C" (Math|Transform|MakeTransform _returnvalue "0, 0, 0" "1.000000,1.000000,1.000000") "Undefined" "MultiplyWithRoot" 0 0)
      (CallFunction|WaitSpecialInteraction 8.0))
    (:NewEnumerator5
      (bind _returnvalue_3 (Game|SpawnActorfromClass "/Game/Blueprints/Interactible/BP_DOTS.BP_DOTS_C" (Math|Transform|MakeTransform _returnvalue "0, 0, 0" "1.000000,1.000000,1.000000") "Undefined" "MultiplyWithRoot" 0 0))
      (Default|ActivateDOTS _returnvalue_3)
      (CallFunction|WaitSpecialInteraction 8.0 _returnvalue_3))))

(fn ManageInteractionsEnd
  (switch Utilities|FlowControl|Switch|SwitchonEPossibleInteractions (Variables|Default|GetLastInteraction)
    (:NewEnumerator2
      (Audio|Components|Audio|Stop (Variables|Default|GetEMFSound)))
    (:NewEnumerator0
      (Components|Activation|Deactivate (Variables|Default|GetNS_Disto))
      (Development|PrintString "Hello"))
    (:NewEnumerator4
      (Rendering|SetVisibility (Variables|Default|GetSpotLight) false false))))

(fn InitializeAI
  (Variables|/Game/Blueprints/AI/WG_DebugInteract.WG_DebugInteract_C|SetCharacterRef (.AsWG%20Debug%20Interact (Utilities|Casting|CastToWG_DebugInteract (UserInterface|GetUserWidgetObject (Variables|Default|GetWidget)))) self)
  (bind _returnvalue (Actor|GetActorOfClass "/Game/Blueprints/Core/BP_Player.BP_Player_C"))
  (Variables|Default|SetPlayerRef _returnvalue)
  (bind _returnvalue_2 (AddComponent|AddAudioComponent false))
  (Variables|Default|SetHeartBeatSanity _returnvalue_2)
  (bind _returnvalue_3 (AddComponent|AddAudioComponent false))
  (bind _output_get (Variables|Default|SetEMFSound _returnvalue_3))
  (Audio|Components|Audio|Stop _output_get))

(fn CheckValidateProof
  (bind _returnvalue (Transformation|GetActorLocation))
  (bind _playerref (Variables|Default|GetPlayerRef))
  (bind _dotsactivated (Variables|Default|GetdotsActivated))
  (bind _playerref_2 (Variables|Default|GetPlayerRef))
  (bind _currentinteraction (Variables|Default|GetCurrentInteraction))
  (bind _proofs (Variables|/Game/Blueprints/Core/BP_Player.BP_Player_C|Getproofs _playerref))
  (bind _proofs_2 (Variables|/Game/Blueprints/Core/BP_Player.BP_Player_C|Getproofs _playerref_2))
  (bind (_value _returnvalue_2) (Utilities|Map|Find _proofs_2 _currentinteraction))
  (Utilities|FlowControl|Sequence
    (:then_0
      (if (and (not _value) _returnvalue_2)
        (switch Utilities|FlowControl|Switch|SwitchonEPossibleInteractions (Variables|Default|GetCurrentInteraction)
          (:NewEnumerator2
            (if (>= (Variables|Default|GetNormalizedDistanceToPlayer) 0.8)
              (Utilities|Map|Add _proofs (Variables|Default|GetCurrentInteraction) true :!label _label)
              (CallFunction|SoundDiscoverProof)))
          (:NewEnumerator0
            (if (Variables|Default|Getb_hasHearedSpirit)
              (goto _label)))
          (:NewEnumerator1
            (if (Variables|Default|GetFreezing)
              (goto _label)))
          (:NewEnumerator4
            (bind _outhit (Collision|SphereTraceForObjects _returnvalue _returnvalue 1.5e+02 (Utilities|Array|MakeArray "ObjectTypeQuery8") false 0 "None"))
            (bind _asbp_door (Utilities|Casting|CastToBP_Door (.hitactor _outhit)))
            (if (Variables|/Game/Blueprints/Interactible/BP_Door.BP_Door_C|Getfingerprinted _asbp_door)
              (Utilities|Map|Add (Variables|/Game/Blueprints/Core/BP_Player.BP_Player_C|Getproofs (Variables|Default|GetPlayerRef)) "NewEnumerator4" true)
              (CallFunction|SoundDiscoverProof)))
          (:NewEnumerator5
            (Utilities|IsValid _dotsactivated
              (:Is%20Valid
                (if (Variables|/Game/Blueprints/Interactible/BP_DOTS.BP_DOTS_C|GethasDetected _dotsactivated)
                  (goto _label))))))))
    (:then_1
      (if (not (.Value (Utilities|Map|Find (Variables|/Game/Blueprints/Core/BP_Player.BP_Player_C|Getproofs (Variables|Default|GetPlayerRef)) "NewEnumerator3")))
        (bind _array_element (Utilities|Array|ForEachLoopwithBreak (Variables|Default|GetbooksActivated) :!label _label_2)
          (:LoopBody
            (if (Variables|/Game/Blueprints/Interactible/BP_Book.BP_Book_C|GetplayerShouldBeDetected _array_element)
              (Utilities|Map|Add _proofs "NewEnumerator3" true)
              (CallFunction|SoundDiscoverProof)
              (goto _label_2 Break))))))))

(fn SoundDiscoverProof
  (bind _returnvalue (Audio|SpawnSound2D "/Game/Audio/Assets/Ghost/Ghost_ClueHit/SC_GHOST_ClueHit.SC_GHOST_ClueHit" 1.0 1.0 0.0 0))
  (Effects|Components|ParticleSystem|SetIntParameter _returnvalue "SwitchFeedbackClue" (Variables|Default|GetshouldPlaySoundGhostFeedbackProof))
  (Math|Integer|IncrementInt (Variables|Default|GetshouldPlaySoundGhostFeedbackProof)
    (:%20%20
      (Audio|Components|Audio|Play _returnvalue 0.0))))

(fn RunAway
  (if (and (Variables|/Game/Blueprints/Core/BP_Player.BP_Player_C|Getb_inUlt (Variables|Default|GetPlayerRef)) (not (Variables|Default|GetHiding)))
    (Variables|Default|SetHiding true)
    (AI|Components|Blackboard|SetValueasBool (AI|GetBlackboard 0) (Utilities|String|StringToName "PlayerUlt") true)
    (Variables|/Script/Engine.CharacterMovementComponent|SetMaxWalkSpeed (Variables|Character|GetCharacterMovement) 6e+02)
    (Utilities|Time|PauseTimerbyHandle (Variables|Default|GetSwitchInteractionHandler))
    (elif (and (not (Variables|/Game/Blueprints/Core/BP_Player.BP_Player_C|Getb_inUlt (Variables|Default|GetPlayerRef))) (Variables|Default|GetHiding))
      (Variables|Default|SetHiding false)
      (AI|Components|Blackboard|SetValueasBool (AI|GetBlackboard 0) (Utilities|String|StringToName "PlayerUlt") false)
      (Variables|/Script/Engine.CharacterMovementComponent|SetMaxWalkSpeed (Variables|Character|GetCharacterMovement) 1.5e+02)
      (Utilities|Time|UnpauseTimerbyHandle (Variables|Default|GetSwitchInteractionHandler)))))

(fn DetermineNewInteraction
  (params (Key :type EPossibleInteractions%20Enum :default "NewEnumerator2"))
  (bind _outactors (Actor|GetAllActorsOfClass "BP_AICharacter_C"))
  (for _array_element _outactors
    (if (.ReturnValue (Utilities|Map|Find (Variables|BP_AICharacter_C|GetInteractions _array_element) Key))
      (return false)))
  (return true))