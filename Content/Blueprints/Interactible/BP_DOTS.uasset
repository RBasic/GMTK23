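; BP_DOTS is a switchable interactible detector that flags the player as detected while AI characters are present.
; An AI overlap volume maintains the list of AI in the room and sets each one's reference to this DOTS, clearing it on exit.
; A player volume tracks players flagged to trigger DOTS.
; Tick latches HasDetected when active with both present; nothing here resets it.
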(event OnComponentBeginOverlap(IADetector)
  (params (OverlappedComponent :type Primitive%20Component%20Object%20Reference) (OtherActor :type Actor%20Object%20Reference) (OtherComp :type Primitive%20Component%20Object%20Reference) (OtherBodyIndex :type Integer) (bFromSweep :type Boolean) (SweepResult :type Hit%20Result%20Structure%20%28by%20ref%29))
  (bind _asbp_aicharacter (Utilities|Casting|CastToBP_AICharacter OtherActor))
  (Utilities|Array|AddUnique (Variables|Default|GetIAInRoom) _asbp_aicharacter)
  (Variables|/Game/Blueprints/AI/BP_AICharacter.BP_AICharacter_C|SetdotsActivated _asbp_aicharacter self))

(event OnComponentEndOverlap(IADetector)
  (params (OverlappedComponent :type Primitive%20Component%20Object%20Reference) (OtherActor :type Actor%20Object%20Reference) (OtherComp :type Primitive%20Component%20Object%20Reference) (OtherBodyIndex :type Integer))
  (bind _asbp_aicharacter (Utilities|Casting|CastToBP_AICharacter OtherActor))
  (if (Utilities|Array|ContainsItem (Variables|Default|GetIAInRoom) OtherActor)
    (Utilities|Array|RemoveItem (Variables|Default|GetIAInRoom) OtherActor)
    (Variables|/Game/Blueprints/AI/BP_AICharacter.BP_AICharacter_C|SetdotsActivated _asbp_aicharacter 0)))

(event OnComponentBeginOverlap(PlayerDetector)
  (params (OverlappedComponent :type Primitive%20Component%20Object%20Reference) (OtherActor :type Actor%20Object%20Reference) (OtherComp :type Primitive%20Component%20Object%20Reference) (OtherBodyIndex :type Integer) (bFromSweep :type Boolean) (SweepResult :type Hit%20Result%20Structure%20%28by%20ref%29))
  (bind _asbp_player (Utilities|Casting|CastToBP_Player OtherActor))
  (if (Variables|/Game/Blueprints/Core/BP_Player.BP_Player_C|Getb_shouldTriggerDOTS _asbp_player)
    (Variables|Default|SetplayerShouldBeDetected true)))

(event OnComponentEndOverlap(PlayerDetector)
  (params (OverlappedComponent :type Primitive%20Component%20Object%20Reference) (OtherActor :type Actor%20Object%20Reference) (OtherComp :type Primitive%20Component%20Object%20Reference) (OtherBodyIndex :type Integer))
  (bind _asbp_player (Utilities|Casting|CastToBP_Player OtherActor))
  (if (Variables|/Game/Blueprints/Core/BP_Player.BP_Player_C|Getb_shouldTriggerDOTS _asbp_player)
    (Variables|Default|SetplayerShouldBeDetected false)))

(event Custom|ActivateDOTS
  (Variables|Default|Setis%20Active true))

(event Custom|DeactivateDOTS
  (Variables|Default|Setis%20Active false))

(event EventBeginPlay)

(event Collision|EventActorBeginOverlap
  (params (OtherActor :type Actor%20Object%20Reference)))

(event EventTick
  (params (DeltaSeconds :type Float%20%28single-precision%29))
  (if (Math|Boolean|ANDBoolean (Variables|Default|Getis%20Active) (Variables|Default|GetplayerShouldBeDetected) (>= (Utilities|Array|Length (Variables|Default|GetIAInRoom)) 1))
    (Variables|Default|SethasDetected true)))

(fn ConstructionScript)