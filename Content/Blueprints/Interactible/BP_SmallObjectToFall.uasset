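; Small physics prop the player can knock or throw so its impact scares nearby AI characters.
; Holding attaches it to the player camera; a click detaches it with an impulse along the camera view if held, otherwise in a random direction.
; The first hit afterward sphere-traces for AI, checks line of sight, and applies a distance-scaled sanity reduction, gated by each AI's fear cooldown.
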(event OnComponentHit(StaticMesh)
  (params (HitComponent :type Primitive%20Component%20Object%20Reference) (OtherActor :type Actor%20Object%20Reference) (OtherComp :type Primitive%20Component%20Object%20Reference) (NormalImpulse :type Vector :default "0, 0, 0") (Hit :type Hit%20Result%20Structure%20%28by%20ref%29))
  (if (Variables|Default|Getb_shouldMakeCreepySound)
    (CallFunction|MakeCreepySound (select (Utilities|Operators|EqualEqual (.normal Hit) "0.000000,0.000000,1.000000" 0.4) (.hitactor Hit) 0))
    (Variables|Default|Setb_shouldMakeCreepySound false)))

(event Custom|MakeCreepySound
  (params ([1] :type Actor%20Object%20Reference))
  (bind _returnvalue (Transformation|GetActorLocation))
  ;[1 1 1] CreepySound
  (bind _outhits (Collision|MultiSphereTraceForObjects _returnvalue _returnvalue (Variables|Default|Getf_radiusCreepySound) (Utilities|Array|MakeArray "ObjectTypeQuery7") false 0 "ForDuration"))
  (for _array_element _outhits
    (bind _asbp_aicharacter (Utilities|Casting|CastToBP_AICharacter (.HitActor (Collision|BreakHitResult _array_element))))
    (bind _returnvalue_2 (Collision|SphereTraceByChannel (Transformation|GetWorldLocation (Variables|Default|GetStaticMesh)) (Transformation|GetActorLocation _asbp_aicharacter) 1e+01 "TraceTypeQuery1" false (Utilities|Array|MakeArray _asbp_aicharacter [1]) "ForDuration"))
    (if (not _returnvalue_2)
      (if (Variables|/Game/Blueprints/AI/BP_AICharacter.BP_AICharacter_C|Getb_canBeAfraidByLittleInteraction _asbp_aicharacter)
        (Default|ManageSanity _asbp_aicharacter "NewEnumerator0" (* (Variables|Default|Getf_littleSanityReduction) (Math|Float|MapRangeClamped (.Distance (Collision|BreakHitResult _array_element)) 0.0 (Variables|Default|Getf_radiusCreepySound) 1.0 0.0)))
        (Variables|/Game/Blueprints/AI/BP_AICharacter.BP_AICharacter_C|Setb_canBeAfraidByLittleInteraction _asbp_aicharacter false)
        (Default|ResetCanbeAfraidOfLittleInteract _asbp_aicharacter)))))

(event Custom|resetHold
  (Utilities|FlowControl|DoOnce false) ; enters at Reset
)

(event EventIsClick
  (params (fromMonster :type Boolean))
  (CallFunction|ResetHold)
  (Physics|SetSimulatePhysics (Variables|Default|GetStaticMesh) true)
  (Transformation|DetachFromActor "KeepWorld" "KeepWorld" "KeepWorld")
  (Physics|AddImpulse (Variables|Default|GetStaticMesh) (* (Math|Vector|SelectVector (Math|Vector|GetForwardVector (Variables|/Game/Blueprints/Core/BP_Player.BP_Player_C|GetCamera (Variables|Default|GetAs%20BP%20Player))) (Math|Random|RandomUnitVector) (Variables|Default|Getb_isHold)) (Variables|Default|Getf_impulseForce)) "None" false)
  (Variables|Default|Setb_shouldMakeCreepySound true))

(event EventIsHold
  (params (since :type Float%20%28double-precision%29) (fromMonster :type Boolean))
  (if (> since 0.2)
    (Utilities|FlowControl|DoOnce false
      (:Completed
        (Physics|SetSimulatePhysics (Variables|Default|GetStaticMesh) false)
        (Transformation|AttachComponentToComponent (Variables|/Game/Blueprints/Core/BP_Player.BP_Player_C|GetCamera (Variables|Default|GetAs%20BP%20Player)) "None" "KeepWorld" "KeepWorld" "KeepWorld" true)
        (Variables|Default|Setb_isHold true)))))

(event EventBeginPlay
  (bind _asbp_player (Utilities|Casting|CastToBP_Player (Game|GetPlayerCharacter 0)))
  (Variables|Default|SetAs%20BP%20Player _asbp_player))

(fn ConstructionScript)