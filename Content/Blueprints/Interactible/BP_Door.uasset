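; Interactive door that toggles open and closed on IsClick, and opens when an AI character overlaps its box while closed.
; A FlipFlop drives a timeline that scrubs the skeletal mesh animation, with monster-triggered closing at double speed plus a ghost slam sound.
; The monster's first use can also reveal one of six random fingerprints.
; MakeCreepySound is empty; its apparent sanity-reduction trace logic is disconnected.
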(event OnComponentBeginOverlap(Box)
  (params (OverlappedComponent :type Primitive%20Component%20Object%20Reference) (OtherActor :type Actor%20Object%20Reference) (OtherComp :type Primitive%20Component%20Object%20Reference) (OtherBodyIndex :type Integer) (bFromSweep :type Boolean) (SweepResult :type Hit%20Result%20Structure%20%28by%20ref%29))
  (Utilities|Casting|CastToBP_AICharacter OtherActor)
  (if (not (Variables|Default|GetOpen))
    (CallFunction|IsClick false false)
    (Development|PrintString (Utilities|GetDisplayName OtherComp))))

(event Custom|MakeCreepySound
  ;[1 1 1] CreepySound
)

(event EventIsClick
  (params (fromMonster :type Boolean) (shouldSpawnFingerprint :type Boolean))
  (bind _skeletalmesh (Variables|Default|GetSkeletalMesh))
  (bind _returnvalue (Transformation|GetWorldLocation _skeletalmesh))
  (Utilities|FlowControl|Sequence
    (:then_0
      (bind _isa (Utilities|FlowControl|FlipFlop)
        (:A
          (Variables|Default|SetOpen _isa)
          (bind (_direction _newtrack_0) (Timeline|Timeline Play)
            (:Update
              (Components|Animation|SetPosition (Variables|Default|GetSkeletalMesh) _newtrack_0 true))
            (:Finished
              (if (and (Utilities|Enum|Equal(Enum) _direction "Backward") fromMonster)
                (Audio|PlaySoundatLocation "/Game/Audio/Assets/Ghost/Ghost_Close_Door_Fast/Ghost_Door_Close_Fast.Ghost_Door_Close_Fast" (Transformation|GetWorldLocation (Variables|Default|GetSkeletalMesh)) "0, 0, 0" 1.0 1.0 0.0 0 0 0 0)
                (CallFunction|MakeCreepySound)))))
        (:B
          (Variables|Default|SetOpen _isa)
          (Components|Timeline|SetPlayRate (Variables|Default|GetTimeline) (Math|Float|SelectFloat 2.0 1.0 fromMonster))
          (Timeline|Timeline Reverse))))
    (:then_1
      (if fromMonster
        (Audio|PlaySoundatLocation "/Game/Audio/Assets/AI/AI_OpenDoors/SC_AI_OpenDoors.SC_AI_OpenDoors" _returnvalue "0, 0, 0" 1.0 1.0 0.0 0 0 0 0)
        (Utilities|FlowControl|DoOnce false
          (:Completed
            (if shouldSpawnFingerprint
              (Development|SetHiddeninGame (.OutItem (Utilities|Array|Random (Utilities|Array|MakeArray (Variables|Default|GetBP_Empreintes1) (Variables|Default|GetBP_Empreintes) (Variables|Default|GetBP_Empreintes2) (Variables|Default|GetBP_Empreintes5) (Variables|Default|GetBP_Empreintes4) (Variables|Default|GetBP_Empreintes3)))) false false)
              (Variables|Default|Setfingerprinted true))))
        (else
          (Audio|PlaySoundatLocation "/Game/Audio/Assets/AI/AI_OpenDoors/SC_AI_OpenDoors.SC_AI_OpenDoors" _returnvalue "0, 0, 0" 1.0 1.0 0.0 0 0 0 0))))))

(fn ConstructionScript)