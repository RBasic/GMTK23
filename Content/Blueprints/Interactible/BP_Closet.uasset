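; BP_Closet is an interactable closet whose two doors toggle open and closed through a flip-flopped timeline rotating them in mirrored yaw.
; Monster clicks double the animation speed and, once the doors finish closing, trigger a creepy sound event.
; That event sphere-traces for nearby AI characters, checks line of sight, applies distance-scaled sanity changes to those able to be scared, then starts their scare reset.
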(event Custom|MakeCreepySound
  (bind _returnvalue (Transformation|GetActorLocation))
  ;[1 1 1] CreepySound
  (bind _outhits (Collision|MultiSphereTraceForObjects _returnvalue _returnvalue (Variables|Default|Getf_radiusCreepySound) (Utilities|Array|MakeArray "ObjectTypeQuery7") false 0 "ForDuration"))
  (for _array_element _outhits
    (bind _asbp_aicharacter (Utilities|Casting|CastToBP_AICharacter (.HitActor (Collision|BreakHitResult _array_element))))
    (bind _returnvalue_2 (Collision|SphereTraceByChannel (Transformation|GetWorldLocation (Variables|Default|GetScene)) (Transformation|GetActorLocation _asbp_aicharacter) 1e+01 "TraceTypeQuery1" false (Utilities|Array|MakeArray _asbp_aicharacter) "ForDuration"))
    (if (not _returnvalue_2)
      (if (Variables|/Game/Blueprints/AI/BP_AICharacter.BP_AICharacter_C|Getb_canBeAfraidByLittleInteraction _asbp_aicharacter)
        (Default|ManageSanity _asbp_aicharacter "NewEnumerator0" (* (Variables|Default|Getf_doorSanityReduction) (Math|Float|MapRangeClamped (.Distance (Collision|BreakHitResult _array_element)) 0.0 (Variables|Default|Getf_radiusCreepySound) 1.0 0.0)))
        (Variables|/Game/Blueprints/AI/BP_AICharacter.BP_AICharacter_C|Setb_canBeAfraidByLittleInteraction _asbp_aicharacter false)
        (Default|ResetCanbeAfraidOfLittleInteract _asbp_aicharacter)))))

(event EventBeginPlay)

(event Collision|EventActorBeginOverlap
  (params (OtherActor :type Actor%20Object%20Reference)))

(event EventTick
  (params (DeltaSeconds :type Float%20%28single-precision%29)))

(event EventIsClick
  (params (fromMonster :type Boolean) (shouldSpawnFingerprint :type Boolean))
  (Components|Timeline|SetPlayRate (Variables|Default|GetTimeline) (select fromMonster 2.0 1.0))
  (Utilities|FlowControl|FlipFlop
    (:A
      (bind (_direction _newtrack_0) (Timeline|Timeline Play)
        (:Update
          (Transformation|SetRelativeRotation (Variables|Default|GetSM_ClosetsDoorA_Door_L) (Math|Rotator|MakeRotator 0.0 0.0 (Math|Float|Lerp 0.0 126.0 _newtrack_0)) false false)
          (Transformation|SetRelativeRotation (Variables|Default|GetSM_ClosetsDoorA_Door_R) (Math|Rotator|MakeRotator 0.0 0.0 (* (Math|Float|Lerp 0.0 126.0 _newtrack_0) -1.0)) false false))
        (:Finished
          (if (and (Utilities|Enum|Equal(Enum) _direction "Backward") fromMonster)
            (CallFunction|MakeCreepySound)))))
    (:B
      (Timeline|Timeline Reverse))))

(fn ConstructionScript)