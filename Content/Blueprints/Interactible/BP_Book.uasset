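; BP_Book is a clickable interactible that affects nearby AI characters' sanity and can flag the player as detected.
; An IADetector overlap volume maintains the list of AI characters in the room.
; A permitted click marks the player as detectable and, through a DoOnce, applies a one-time sanity change to those AI.
; Tick sets HasDetected while the book is active, the player is detectable and any AI is present.
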(event OnComponentBeginOverlap(IADetector)
  (params (OverlappedComponent :type Primitive%20Component%20Object%20Reference) (OtherActor :type Actor%20Object%20Reference) (OtherComp :type Primitive%20Component%20Object%20Reference) (OtherBodyIndex :type Integer) (bFromSweep :type Boolean) (SweepResult :type Hit%20Result%20Structure%20%28by%20ref%29))
  (bind _asbp_aicharacter (Utilities|Casting|CastToBP_AICharacter OtherActor))
  (Utilities|Array|AddUnique (Variables|Default|GetIAInRoom) _asbp_aicharacter))

(event OnComponentEndOverlap(IADetector)
  (params (OverlappedComponent :type Primitive%20Component%20Object%20Reference) (OtherActor :type Actor%20Object%20Reference) (OtherComp :type Primitive%20Component%20Object%20Reference) (OtherBodyIndex :type Integer))
  (if (Utilities|Array|ContainsItem (Variables|Default|GetIAInRoom) OtherActor)
    (Utilities|Array|RemoveItem (Variables|Default|GetIAInRoom) OtherActor)))

(event Custom|ActivateBook
  (Variables|Default|SetisActiv true))

(event Custom|DeactivateBook
  (Variables|Default|SetisActiv false))

(event EventTick
  (params (DeltaSeconds :type Float%20%28single-precision%29))
  (if (Math|Boolean|ANDBoolean (Variables|Default|GetisActiv) (Variables|Default|GetplayerShouldBeDetected) (>= (Utilities|Array|Length (Variables|Default|GetIAInRoom)) 1))
    (Variables|Default|SethasDetected true)))

(event EventIsClick
  (params (fromMonster :type Boolean) (shouldSpawnFingerprint :type Boolean))
  (bind _asbp_player (Utilities|Casting|CastToBP_Player (Game|GetPlayerCharacter 0)))
  (if (Variables|/Game/Blueprints/Core/BP_Player.BP_Player_C|Getb_canInteractWithBook _asbp_player)
    (Variables|Default|SetplayerShouldBeDetected true)
    (Utilities|FlowControl|DoOnce false
      (:Completed
        (for _array_element (Variables|Default|GetIAInRoom)
          (bind _asbp_aicharacter (Utilities|Casting|CastToBP_AICharacter _array_element))
          (Default|ManageSanity _asbp_aicharacter "NewEnumerator0" 0.15))))))

(fn ConstructionScript)