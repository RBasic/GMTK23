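; BP_GameLoopManager evaluates the game's win and lose conditions and ends the session.
; CheckWin succeeds when every BP_AICharacter is dead, while CheckLose triggers when every value in BP_Player's Proofs map is true.
; Either outcome stores IsThisWin on BP_CustomGameInstance, so the result survives the level change, then opens the Menu level.
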(event Custom|CheckWin
  (bind _outactors (Actor|GetAllActorsOfClass "/Game/Blueprints/AI/BP_AICharacter.BP_AICharacter_C"))
  (Variables|Default|SetthisIsWin true)
  (bind _array_element (Utilities|Array|ForEachLoopwithBreak _outactors :!label _label)
    (:LoopBody
      (if (not (Variables|/Game/Blueprints/AI/BP_AICharacter.BP_AICharacter_C|GetIsDead _array_element))
        (Variables|Default|SetthisIsWin false)
        (goto _label Break)))
    (:Completed
      (if (Variables|Default|GetthisIsWin)
        (bind _asbp_custom_game_instance (Utilities|Casting|CastToBP_CustomGameInstance (Game|GetGameInstance)))
        (Variables|/Game/Blueprints/Core/BP_CustomGameInstance.BP_CustomGameInstance_C|SetisThisWin? _asbp_custom_game_instance true)
        (Game|OpenLevel(byObjectReference) "/Game/Maps/Menu.Menu")))))

(event Custom|CheckLose
  (bind _returnvalue (Actor|GetActorOfClass "/Game/Blueprints/Core/BP_Player.BP_Player_C"))
  (bind _values (Utilities|Map|Values (Variables|/Game/Blueprints/Core/BP_Player.BP_Player_C|Getproofs _returnvalue)))
  (Variables|Default|SetthisIsLose true)
  (bind _array_element (Utilities|Array|ForEachLoopwithBreak _values :!label _label)
    (:LoopBody
      (if (not _array_element)
        (Variables|Default|SetthisIsLose false)
        (goto _label Break)))
    (:Completed
      (if (Variables|Default|GetthisIsLose)
        (bind _asbp_custom_game_instance (Utilities|Casting|CastToBP_CustomGameInstance (Game|GetGameInstance)))
        (Variables|/Game/Blueprints/Core/BP_CustomGameInstance.BP_CustomGameInstance_C|SetisThisWin? _asbp_custom_game_instance false)
        (Game|OpenLevel(byObjectReference) "/Game/Maps/Menu.Menu")))))

(fn ConstructionScript)