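; Player pawn for the monster, haunting AI investigators with abilities from the type chosen in the game instance.
; DT_Monsters supplies three proofs that enable evidence such as EMF, orbs, freezing or fingerprints, alongside trace-based interaction and spirit box screams.
; Tick emphasizes the closest investigator's heartbeat and charges the ultimate from living investigators' average insanity.
; A full gauge triggers a timeline-driven ultimate with camera shake, faster movement and hidden fog and post-process.
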(event Custom|breakLoopInteract
  ;[1 1 1] Interact
  (Utilities|Array|ForEachLoopwithBreak (stale _outhits)) ; enters at Break
)

(event Custom|isMonster
  (params (isTypeOf :type Name))
  (bind _as_bp_custom_player_controller (Variables|Default|GetAs%20BP%20Custom%20Player%20Controller))
  (bind _proofs (Variables|Default|Getproofs))
  (bind _returnvalue (Utilities|GetDataTableRow "/Game/Blueprints/DT_Monsters.DT_Monsters" isTypeOf)
    (:then
      (bind _output_get (Variables|Default|SetisMonsterType (Utilities|Struct|MakeS_Monster (.description _returnvalue) (.proof1 _returnvalue) (.proof2 _returnvalue) (.proof3 _returnvalue))))
      (Development|PrintString (Utilities|String|Append "p1 :" (Utilities|String|EnumtoString (.proof1 _output_get)) "-> p2 :" (Utilities|String|EnumtoString (.proof2 _output_get)) "-> p3 :" (Utilities|String|EnumtoString (.proof3 _output_get))))
      (CallFunction|EMFSelectRandomLevel)
      (CallFunction|TriggerProofPassiv)
      (Variables|Default|Setb_hasChooseMonster true)
      (Input|SetInputModeGameOnly _as_bp_custom_player_controller true)
      (Variables|/Script/Engine.PlayerController|SetbShowMouseCursor _as_bp_custom_player_controller false)
      (Utilities|Map|Add _proofs (.proof1 (Variables|Default|GetisMonsterType)) false)
      (Utilities|Map|Add _proofs (.proof2 (Variables|Default|GetisMonsterType)) false)
      (Utilities|Map|Add _proofs (.proof3 (Variables|Default|GetisMonsterType)) false)
      (bind _outactors (Actor|GetAllActorsOfClass "/Game/Blueprints/AI/BP_AICharacter.BP_AICharacter_C"))
      (bind _output_get_2 (Variables|Default|SetIA_Character _outactors))
      (for _array_element _output_get_2
        (Default|PlayerIsActive _array_element))
      (Variables|Default|SetIncreaseUlti true))))

(event Custom|ResetStopUltFeedback
  (Utilities|FlowControl|DoOnce false) ; enters at Reset
)

(event Custom|SetFeedBackUlt
  (Utilities|FlowControl|Sequence
    (:then_0
      (CallFunction|ResetStopUltFeedback))
    (:then_1
      (Utilities|FlowControl|DoOnce false
        (:Completed
          (Utilities|FlowControl|Sequence
            (:then_0
              (CameraShake|Start (Variables|Default|GetCameraShakeSource))
              (Variables|Default|SetIncreaseUlti false)
              (Variables|Default|Setb_inUlt true)
              (bind _newtrack_0 (Timeline|Timeline PlayFromStart)
                (:Update
                  (CallFunction|UltimateGaugeManager "NewEnumerator4" _newtrack_0))
                (:Finished
                  (CallFunction|StopFeedBackUlt))))
            (:then_1
              (Variables|Default|SetfeedbackUltForward? true)
              (bind _returnvalue (Actor|GetActorOfClass "/Script/Engine.PostProcessVolume"))
              (Variables|Default|SetpostProRef _returnvalue)
              (if (Variables|Default|GetfeedbackUltForward?)
                (Utilities|FlowControl|Delay 0.25)
                (bind _returnvalue_2 (Actor|GetActorOfClass "/Script/Engine.ExponentialHeightFog"))
                (Rendering|SetActorHiddenInGame _returnvalue_2 true)
                (Rendering|SetActorHiddenInGame (Variables|Default|GetpostProRef) true)
                (bind _returnvalue_3 (Actor|GetActorOfClass "/Game/Blueprints/Core/BP_Spider.BP_Spider_C"))
                (Development|SetHiddeninGame (Variables|/Game/Blueprints/Core/BP_Spider.BP_Spider_C|GetNiagara _returnvalue_3) true false)
                (bind _newtrack_0_2 (Timeline|Timeline_0 Play)
                  (:Update
                    (Variables|/Script/Engine.CharacterMovementComponent|SetMaxWalkSpeed (Variables|Character|GetCharacterMovement) (Math|Float|Lerp 2e+02 4e+02 _newtrack_0_2))))
                (else
                  (bind _returnvalue_4 (Actor|GetActorOfClass "/Script/Engine.ExponentialHeightFog"))
                  (Rendering|SetActorHiddenInGame _returnvalue_4 false)
                  (Rendering|SetActorHiddenInGame (Variables|Default|GetpostProRef) false)
                  (bind _returnvalue_5 (Actor|GetActorOfClass "/Game/Blueprints/Core/BP_Spider.BP_Spider_C"))
                  (Development|SetHiddeninGame (Variables|/Game/Blueprints/Core/BP_Spider.BP_Spider_C|GetNiagara _returnvalue_5) false false)
                  (Timeline|Timeline_0 Reverse))))))))))

(event Custom|StopFeedBackUlt
  (Utilities|FlowControl|Sequence
    (:then_0
      (CallFunction|ResetStartUltFeedback))
    (:then_1
      (Utilities|FlowControl|DoOnce false
        (:Completed
          (Utilities|FlowControl|Sequence
            (:then_0
              (Variables|Default|SetfeedbackUltForward? false)
              (bind _returnvalue (Actor|GetActorOfClass "/Script/Engine.PostProcessVolume"))
              (Variables|Default|SetpostProRef _returnvalue)
              (if (Variables|Default|GetfeedbackUltForward?)
                (Utilities|FlowControl|Delay 0.25)
                (bind _returnvalue_2 (Actor|GetActorOfClass "/Script/Engine.ExponentialHeightFog"))
                (Rendering|SetActorHiddenInGame _returnvalue_2 true)
                (Rendering|SetActorHiddenInGame (Variables|Default|GetpostProRef) true)
                (bind _returnvalue_3 (Actor|GetActorOfClass "/Game/Blueprints/Core/BP_Spider.BP_Spider_C"))
                (Development|SetHiddeninGame (Variables|/Game/Blueprints/Core/BP_Spider.BP_Spider_C|GetNiagara _returnvalue_3) true false)
                (bind _newtrack_0 (Timeline|Timeline_0 Play)
                  (:Update
                    (Variables|/Script/Engine.CharacterMovementComponent|SetMaxWalkSpeed (Variables|Character|GetCharacterMovement) (Math|Float|Lerp 2e+02 4e+02 _newtrack_0))))
                (else
                  (bind _returnvalue_4 (Actor|GetActorOfClass "/Script/Engine.ExponentialHeightFog"))
                  (Rendering|SetActorHiddenInGame _returnvalue_4 false)
                  (Rendering|SetActorHiddenInGame (Variables|Default|GetpostProRef) false)
                  (bind _returnvalue_5 (Actor|GetActorOfClass "/Game/Blueprints/Core/BP_Spider.BP_Spider_C"))
                  (Development|SetHiddeninGame (Variables|/Game/Blueprints/Core/BP_Spider.BP_Spider_C|GetNiagara _returnvalue_5) false false)
                  (Timeline|Timeline_0 Reverse))))
            (:then_1
              (Variables|Default|Setb_inUlt false)
              (CameraShake|StopAllCameraShakes (Variables|Default|GetCameraShakeSource) true)
              (Variables|Default|SetIncreaseUlti true))))))))

(event Custom|IncreaseUltimateGauge
  (if (Variables|Default|GetIncreaseUlti)
    (Variables|Default|Setf_sanityGlobal 0.0)
    (Variables|Default|Seti_playersActive 0)
    (for _array_element (Variables|Default|GetIA_Character)
      (if (not (Variables|/Game/Blueprints/AI/BP_AICharacter.BP_AICharacter_C|GetIsDead _array_element))
        (Variables|Default|Setf_sanityGlobal (+ (Variables|Default|Getf_sanityGlobal) (Variables|/Game/Blueprints/AI/BP_AICharacter.BP_AICharacter_C|GetInsanity _array_element)))
        (Math|Integer|IncrementInt (Variables|Default|Geti_playersActive))))
    (Variables|Default|Setf_sanityGlobal (/ (Variables|Default|Getf_sanityGlobal) (Variables|Default|Geti_playersActive)))
    (bind _output_get (CallFunction|UltimateGaugeManager "NewEnumerator0" (* (Variables|Default|Getf_sanityGlobal) (Variables|Default|Getf_muliplicatorUltimate))))
    (if (== _output_get (Variables|Default|Getf_ultimateGauge_Max))
      (CallFunction|SetFeedBackUlt))))

(event Custom|TriggerProofPassiv
  (bind _ismonstertype (Variables|Default|GetisMonsterType))
  (CallFunction|FreezingDeactive)
  (Utilities|FlowControl|Sequence
    (:then_0
      (switch Utilities|FlowControl|Switch|SwitchonEPossibleInteractions (.proof1 _ismonstertype)
        (:NewEnumerator2
          (CallFunction|EMFMakeSoundActivate))
        (:NewEnumerator6
          (CallFunction|ActivateSpawnOrb))
        (:NewEnumerator1
          (CallFunction|FreezingActive))
        (:NewEnumerator4
          (Variables|Default|Setb_shouldSpawnFingerPrint true))
        (:NewEnumerator3
          (Variables|Default|Setb_canInteractWithBook true))
        (:NewEnumerator5
          (Variables|Default|Setb_shouldTriggerDOTS true))))
    (:then_1
      (switch Utilities|FlowControl|Switch|SwitchonEPossibleInteractions (.proof2 _ismonstertype)
        (:NewEnumerator2
          (CallFunction|EMFMakeSoundActivate))
        (:NewEnumerator6
          (CallFunction|ActivateSpawnOrb))
        (:NewEnumerator1
          (CallFunction|FreezingActive))
        (:NewEnumerator4
          (Variables|Default|Setb_shouldSpawnFingerPrint true))
        (:NewEnumerator3
          (Variables|Default|Setb_canInteractWithBook true))
        (:NewEnumerator5
          (Variables|Default|Setb_shouldTriggerDOTS true))))
    (:then_2
      (switch Utilities|FlowControl|Switch|SwitchonEPossibleInteractions (.proof3 _ismonstertype)
        (:NewEnumerator2
          (CallFunction|EMFMakeSoundActivate))
        (:NewEnumerator6
          (CallFunction|ActivateSpawnOrb))
        (:NewEnumerator1
          (CallFunction|FreezingActive))
        (:NewEnumerator4
          (Variables|Default|Setb_shouldSpawnFingerPrint true))
        (:NewEnumerator3
          (Variables|Default|Setb_canInteractWithBook true))
        (:NewEnumerator5
          (Variables|Default|Setb_shouldTriggerDOTS true))))))

(event Custom|receiveHeartBeatSound
  (for (_array_element _array_index) (Variables|Default|GetIA_Character)
    (if (== _array_index 0)
      (Variables|Default|SetMinDist (Math|Vector|Distance(Vector) (Transformation|GetActorLocation _array_element) (Transformation|GetActorLocation)) :!label _label)
      (Variables|Default|SetIndexClosest _array_index)
      (elif (<= (Math|Vector|Distance(Vector) (Transformation|GetActorLocation _array_element) (Transformation|GetActorLocation)) (Variables|Default|GetMinDist))
        (goto _label))))
  (for (_array_element_2 _array_index_2) (Variables|Default|GetIA_Character)
    (Audio|Components|Audio|AdjustVolume (Variables|/Game/Blueprints/AI/BP_AICharacter.BP_AICharacter_C|GetHeartBeatSanity _array_element_2) 0.0 (select (== _array_index_2 (Variables|Default|GetIndexClosest)) 1.0 0.05) "Linear" :!class /Script/Engine.AudioComponent)))

(event Custom|SetFXBook
  (params (InValue :type Vector))
  (bind _ns_book (Variables|Default|GetNS_Book))
  (Niagara|SetNiagaraVariable(Vector3) _ns_book "End" InValue)
  (Components|Activation|Activate _ns_book true))

(event Custom|ResetStartUltFeedback
  (Utilities|FlowControl|DoOnce false) ; enters at Reset
)

(event Input|EnhancedActionEvents|EnhancedInputActionIA_Move
  (params (ActionValue :type Vector%202D%20Structure) (ElapsedSeconds :type Float%20%28double-precision%29) (TriggeredSeconds :type Float%20%28double-precision%29) (InputAction :type Input%20Action%20Object%20Reference :default "/Game/Inputs/Actions/IA_Move.IA_Move"))
  (bind _f_movespeed (Variables|Default|Getf_moveSpeed))
  ;[1 1 1] BasicCharaMove
  (:Triggered
    (if (Variables|Default|Getb_hasChooseMonster)
      (Utilities|FlowControl|Sequence
        (:then_0
          (Pawn|Input|AddMovementInput (Math|Vector|GetForwardVector (Variables|Default|GetCamera)) (* (.y ActionValue) _f_movespeed) false))
        (:then_1
          (Pawn|Input|AddMovementInput (Math|Vector|GetRightVector (Variables|Default|GetCamera)) (* (.x ActionValue) _f_movespeed) false))))))

(event Input|EnhancedActionEvents|EnhancedInputActionIA_Look
  (params (ActionValue :type Vector%202D%20Structure) (ElapsedSeconds :type Float%20%28double-precision%29) (TriggeredSeconds :type Float%20%28double-precision%29) (InputAction :type Input%20Action%20Object%20Reference :default "/Game/Inputs/Actions/IA_Look.IA_Look"))
  (bind _as_bp_custom_player_controller (Variables|Default|GetAs%20BP%20Custom%20Player%20Controller))
  (bind _f_mousesensitivity (Variables|/Game/Blueprints/Core/BP_CustomPlayerController.BP_CustomPlayerController_C|Getf_mouseSensitivity _as_bp_custom_player_controller))
  ;[1 1 1] BasicCharaMove
  (:Triggered
    (if (Variables|Default|Getb_hasChooseMonster)
      (Utilities|FlowControl|Sequence
        (:then_0
          (Pawn|Input|AddControllerYawInput (* (.x ActionValue) _f_mousesensitivity)))
        (:then_1
          (Pawn|Input|AddControllerPitchInput (* (.y ActionValue) _f_mousesensitivity)))))))

(event Input|EnhancedActionEvents|EnhancedInputActionIA_Interact
  (params (ActionValue :type Boolean) (ElapsedSeconds :type Float%20%28double-precision%29) (TriggeredSeconds :type Float%20%28double-precision%29) (InputAction :type Input%20Action%20Object%20Reference :default "/Game/Inputs/Actions/IA_Interact.IA_Interact"))
  (bind _camera (Variables|Default|GetCamera))
  (bind _returnvalue (Transformation|GetWorldLocation _camera))
  ;[1 1 1] Interact
  (:Triggered
    (Utilities|IsValid (Variables|Default|Geta_actorHold)
      (:Is%20Valid
        (Class|BPIInteract|IsHold(Message) (Variables|Default|Geta_actorHold) TriggeredSeconds true))))
  (:Started
    (bind _outhit (Collision|SphereTraceByChannel _returnvalue (+ _returnvalue (* (Math|Vector|GetForwardVector _camera) (Variables|Default|Getf_interactRange))) (Variables|Default|Getf_interactRadius) "TraceTypeQuery3" false 0 "None"))
    (if (.bblockinghit _outhit)
      (Variables|Default|Seta_actorHold (.hitactor _outhit))
      (Utilities|Casting|CastToBP_AICharacter (.hitactor _outhit)))
    (CallFunction|MakeScreamSpiritBox))
  (:Completed
    (Utilities|IsValid (Variables|Default|Geta_actorHold)
      (:Is%20Valid
        (Class|BPIInteract|IsClick(Message) (Variables|Default|Geta_actorHold) true (Variables|Default|Getb_shouldSpawnFingerPrint))
        (Variables|Default|Seta_actorHold 0)))))

(event Input|EnhancedActionEvents|EnhancedInputActionIA_TalkBack
  (params (ActionValue :type Boolean) (ElapsedSeconds :type Float%20%28double-precision%29) (TriggeredSeconds :type Float%20%28double-precision%29) (InputAction :type Input%20Action%20Object%20Reference :default "/Game/Inputs/Actions/IA_TalkBack.IA_TalkBack"))
  (:Triggered
    (CallFunction|MakeScreamSpiritBox))
  (:Completed
    (Utilities|FlowControl|Delay 0.2)
    (for _array_element (Variables|Default|GetIA_Character)
      (Variables|/Game/Blueprints/AI/BP_AICharacter.BP_AICharacter_C|SethearedSpiritBox _array_element false))))

(event EventBeginPlay
  (Utilities|FlowControl|Sequence
    (:then_0
      (bind _returnvalue (Rendering|Material|CreateDynamicMaterialInstance "/Game/Materials/PP/PP_Frozen.PP_Frozen" "None" "None" :!class /Script/Engine.KismetMaterialLibrary))
      (bind _output_get (Variables|Default|SetFrozenPP _returnvalue))
      (Utilities|Struct|SetmembersinPostProcessSettings (Variables|/Script/Engine.CameraComponent|GetPostProcessSettings (Variables|Default|GetCamera)) (Utilities|Struct|MakeWeightedBlendables (Utilities|Array|MakeArray (Utilities|Struct|MakeWeightedBlendable 1.0 _output_get)))))
    (:then_1
      (bind _returnvalue_2 (UserInterface|CreateWidget "/Game/Widget/W_Interface.W_Interface_C"))
      (bind _output_get_2 (Variables|Default|Setwid_refInGame _returnvalue_2))
      (Variables|/Game/Widget/W_Interface.W_Interface_C|SetplayerRef _output_get_2 self)
      (UserInterface|Viewport|AddtoViewport _output_get_2 0)
      (bind _asbp_custom_game_instance (Utilities|Casting|CastToBP_CustomGameInstance (Game|GetGameInstance)))
      (CallFunction|IsMonster (Utilities|String|StringToName (Utilities|String|ToString(Text) (Variables|/Game/Blueprints/Core/BP_CustomGameInstance.BP_CustomGameInstance_C|GetChosenMonster _asbp_custom_game_instance)))))))

(event EventTick
  (params (DeltaSeconds :type Float%20%28single-precision%29))
  (CallFunction|ReceiveHeartBeatSound)
  (CallFunction|IncreaseUltimateGauge))

(event EventPossessed
  (params (NewController :type Controller%20Object%20Reference))
  (bind _asbp_custom_player_controller (Utilities|Casting|CastToBP_CustomPlayerController NewController))
  (Variables|Default|SetAs%20BP%20Custom%20Player%20Controller _asbp_custom_player_controller)
  (CallFunction|UltimateGaugeManager "NewEnumerator3" 1.0)
  (CallFunction|UltimateGaugeManager "NewEnumerator4" 0.0)
  (Input|SetInputModeGameandUI (Variables|Default|GetAs%20BP%20Custom%20Player%20Controller) 0 "DoNotLock" true true))

(event OnComponentBeginOverlap(FreezingZone)
  (params (OverlappedComponent :type Primitive%20Component%20Object%20Reference) (OtherActor :type Actor%20Object%20Reference) (OtherComp :type Primitive%20Component%20Object%20Reference) (OtherBodyIndex :type Integer) (bFromSweep :type Boolean) (SweepResult :type Hit%20Result%20Structure%20%28by%20ref%29))
  ;[1 1 1] FreezeInteraction
  (bind _asbp_aicharacter (Utilities|Casting|CastToBP_AICharacter OtherActor))
  (bind _returnvalue (Utilities|Time|SetTimerbyEvent (delegate Custom|CheckFreeze) (Utilities|Time|GetWorldDeltaSeconds) true))
  (Variables|Default|Setth_handlerFreeze _returnvalue)
  (Utilities|Array|AddUnique (Variables|Default|Geta_CharacterFreezed) _asbp_aicharacter))

(event OnComponentEndOverlap(FreezingZone)
  (params (OverlappedComponent :type Primitive%20Component%20Object%20Reference) (OtherActor :type Actor%20Object%20Reference) (OtherComp :type Primitive%20Component%20Object%20Reference) (OtherBodyIndex :type Integer))
  ;[1 1 1] FreezeInteraction
  (bind _asbp_aicharacter (Utilities|Casting|CastToBP_AICharacter OtherActor))
  (if (Utilities|Array|ContainsItem (Variables|Default|Geta_CharacterFreezed) _asbp_aicharacter)
    (Utilities|Array|RemoveItem (Variables|Default|Geta_CharacterFreezed) _asbp_aicharacter)
    (Variables|/Game/Blueprints/AI/BP_AICharacter.BP_AICharacter_C|SetFreezing _asbp_aicharacter false)
    (if (< (Utilities|Array|Length (Variables|Default|Geta_CharacterFreezed)) 1)
      (Utilities|Time|ClearandInvalidateTimerbyHandle (Variables|Default|Getth_handlerFreeze)))))

(event OnComponentBeginOverlap(Sphere)
  (params (OverlappedComponent :type Primitive%20Component%20Object%20Reference) (OtherActor :type Actor%20Object%20Reference) (OtherComp :type Primitive%20Component%20Object%20Reference) (OtherBodyIndex :type Integer) (bFromSweep :type Boolean) (SweepResult :type Hit%20Result%20Structure%20%28by%20ref%29))
  (Utilities|Casting|CastToBP_Camera OtherActor)
  (Variables|Default|Setb_isSeenByCamera true))

(event OnComponentEndOverlap(Sphere)
  (params (OverlappedComponent :type Primitive%20Component%20Object%20Reference) (OtherActor :type Actor%20Object%20Reference) (OtherComp :type Primitive%20Component%20Object%20Reference) (OtherBodyIndex :type Integer))
  (Utilities|Casting|CastToBP_Camera OtherActor)
  (Variables|Default|Setb_isSeenByCamera false))

(event Custom|FreezingActive
  ;[1 1 1] FreezeInteraction
  (Collision|SetCollisionResponsetoChannel (Variables|Default|GetFreezingZone) "ECC_GameTraceChannel2" "ECR_Overlap")
  (Rendering|Material|SetScalarParameterValue (Variables|Default|GetFrozenPP) "Opacity" 1.0 :!class /Script/Engine.MaterialInstanceDynamic))

(event Custom|FreezingDeactive
  ;[1 1 1] FreezeInteraction
  (Collision|SetCollisionResponsetoChannel (Variables|Default|GetFreezingZone) "ECC_GameTraceChannel2" "ECR_Ignore")
  (Rendering|Material|SetScalarParameterValue (Variables|Default|GetFrozenPP) "Opacity" 0.0 :!class /Script/Engine.MaterialInstanceDynamic))

(event Custom|ActivateSpawnOrb
  ;[1 1 1] OrbSpawn
  (bind _returnvalue (Utilities|Time|SetTimerbyEvent (delegate Custom|SpawnOrb) 2.2 true))
  (Variables|Default|Setth_orbHandler _returnvalue))

(event Custom|EMFMakeSoundActivate
  ;[1 1 1] EMF SoundSelection
  (Variables|Default|Seti_EMFSoundMax 5))

(event Custom|EMFSelectRandomLevel
  ;[1 1 1] EMF SoundSelection
  (Variables|Default|Seti_EMFSoundMax (Math|Random|RandomIntegerinRange 0 4)))

(event Custom|DeactivateSpawnOrb
  ;[1 1 1] OrbSpawn
  (if (Utilities|Time|IsValidTimerHandle (Variables|Default|Getth_orbHandler))
    (Utilities|Time|ClearandInvalidateTimerbyHandle (Variables|Default|Getth_orbHandler))))

(event Custom|SpawnOrb
  ;[1 1 1] OrbSpawn
  (if (>= (Math|Vector|VectorLength (Variables|/Script/Engine.MovementComponent|GetVelocity (Variables|Character|GetCharacterMovement))) 3e+02)
    (Game|SpawnActorfromClass "/Game/Blueprints/Core/BP_Orb.BP_Orb_C" (Transformation|GetActorTransform) "Undefined" "MultiplyWithRoot" 0 self 0)
    (if (Variables|Default|Getb_isSeenByCamera)
      (Variables|Default|Setb_willBeDetectedByCamera true))))

(event Custom|makeScream_SpiritBox
  ;[1 1 1] SpiritBox
  (if (not (Variables|Default|Getscreaming))
    (Audio|PlaySound2D "/Game/Audio/Assets/Ghost/Ghost_Vox_Hunting/Ghost_Kill_IA.Ghost_Kill_IA" 1.0 1.0 0.0 0 0)
    (Variables|Default|Setscreaming (.ReturnValue (Utilities|Map|Find (Variables|Default|Getproofs) "NewEnumerator0")))
    (Utilities|FlowControl|Delay 2.0)
    (Variables|Default|Setscreaming false)))

(event Custom|CheckFreeze
  ;[1 1 1] FreezeInteraction
  (for _array_element (Variables|Default|Geta_CharacterFreezed)
    (bind _returnvalue (Collision|SphereTraceByChannel (Transformation|GetActorLocation _array_element) (Transformation|GetActorLocation) 1e+01 "TraceTypeQuery1" false (Utilities|Array|MakeArray _array_element) "None"))
    (Variables|/Game/Blueprints/AI/BP_AICharacter.BP_AICharacter_C|SetFreezing _array_element (not _returnvalue))))

(fn ConstructionScript)

(fn UltimateGaugeManager
  (params (State :type E_fManagerState%20Enum :default "NewEnumerator0") (Value :type Float%20%28double-precision%29))
  (switch Utilities|FlowControl|Switch|SwitchonE_fManagerState State
    (:NewEnumerator0
      (Variables|Default|Setf_ultimateGauge (Math|Float|MapRangeClamped (+ (Variables|Default|Getf_ultimateGauge) Value) 0.0 (Variables|Default|Getf_ultimateGauge_Max) 0.0 1.0)))
    (:NewEnumerator1
      _)
    (:NewEnumerator4
      (Variables|Default|Setf_ultimateGauge (Math|Float|MapRangeClamped Value 0.0 (Variables|Default|Getf_ultimateGauge_Max) 0.0 1.0)))
    (:NewEnumerator2
      (Variables|Default|Setf_ultimateGauge 0.0))
    (:NewEnumerator3
      (Variables|Default|Setf_ultimateGauge_Max Value)))
  (return (Variables|Default|Getf_ultimateGauge)))