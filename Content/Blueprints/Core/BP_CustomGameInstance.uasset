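; BP_CustomGameInstance is a Game Instance Blueprint that switches the player's input between QWERTY and AZERTY keyboard layouts.
; SwitchQwerty flips the Qwerty flag, then calls RefreshMapping to apply the change.
; RefreshMapping gets player 0's BP_CustomPlayerController, clears all Enhanced Input mappings and adds either IMC_Qwerty or IMC_Azerty based on the flag.
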(fn SwitchQwerty
  (Variables|Default|SetQwerty (not (Variables|Default|GetQwerty)))
  (CallFunction|RefreshMapping))

(fn RefreshMapping
  (bind _asbp_custom_player_controller (Utilities|Casting|CastToBP_CustomPlayerController (Game|GetPlayerController 0)))
  (Class|EnhancedInputSubsystemInterface|ClearAllMappings (PlayerController|LocalPlayerSubsystems|GetEnhancedInputLocalPlayerSubsystem _asbp_custom_player_controller))
  (Input|AddMappingContext (PlayerController|LocalPlayerSubsystems|GetEnhancedInputLocalPlayerSubsystem _asbp_custom_player_controller) (select (Variables|Default|GetQwerty) "/Game/Inputs/IMC_Qwerty.IMC_Qwerty" "/Game/Inputs/IMC_Azerty.IMC_Azerty") 0 "(bIgnoreAllPressedKeysUntilRelease=True,bForceImmediately=False)"))