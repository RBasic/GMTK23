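; Player controller that handles the game's pause toggle and refreshes input mapping when it possesses a pawn.
; On possess it calls RefreshMapping on the custom game instance.
; The IA_Pause input toggles pause, lazily creating and reusing the WG_PauseMenu widget and switching cursor visibility and input mode.
; A ResumeGame event shares the unpause path, removing the menu and restoring game-only input.
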(event Custom|ResumeGame
  (Game|SetGamePaused false)
  (Widget|RemovefromParent (Variables|Default|GetPauseMenu))
  (Variables|Default|SetbShowMouseCursor false)
  (Input|SetInputModeGameOnly self true))

(event Input|EnhancedActionEvents|EnhancedInputActionIA_Pause
  (params (ActionValue :type Boolean) (ElapsedSeconds :type Float%20%28double-precision%29) (TriggeredSeconds :type Float%20%28double-precision%29) (InputAction :type Input%20Action%20Object%20Reference :default "/Game/Inputs/Actions/IA_Pause.IA_Pause"))
  (:Started
    (if (Game|IsGamePaused)
      (Game|SetGamePaused false)
      (Widget|RemovefromParent (Variables|Default|GetPauseMenu))
      (Variables|Default|SetbShowMouseCursor false)
      (Input|SetInputModeGameOnly self true)
      (else
        (Game|SetGamePaused true)
        (Variables|Default|GetPauseMenu
          (:then
            _)
          (:else
            (bind _returnvalue (UserInterface|CreateWidget "/Game/Widget/WG_PauseMenu.WG_PauseMenu_C" (Game|GetPlayerController 0)))
            (Variables|Default|SetPauseMenu _returnvalue)))
        (UserInterface|Viewport|AddtoViewport (Variables|Default|GetPauseMenu) 0)
        (Variables|Default|SetbShowMouseCursor true)
        (Input|SetInputModeGameandUI self (Variables|Default|GetPauseMenu) "DoNotLock" false true)))))

(event EventBeginPlay)

(event EventTick
  (params (DeltaSeconds :type Float%20%28single-precision%29)))

(event EventPossess
  (params (PossessedPawn :type Pawn%20Object%20Reference))
  (Default|RefreshMapping (.AsBP%20Custom%20Game%20Instance (Utilities|Casting|CastToBP_CustomGameInstance (Game|GetGameInstance)))))

(fn ConstructionScript)